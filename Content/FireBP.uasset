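; Fire hazard actor that plays a fire sound on spawn and damages players standing inside its Box.
; A self-calling Hit event, started at BeginPlay, polls overlapping players every 0.1 seconds and applies Damage through PlayerTakeDamage.
; The Box begin-overlap handler only casts to the player, as its damage call is disconnected.
; Spawn count, life and creation time are initialized but not used in these graphs.
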(event `self.ReceiveBeginPlay`
  (set `self.maxNbSpawn` 4)
  (set `self.maxLife` 100)
  (set `self.timeToCreate` 10.0)
  (set `self.damage` 1)
  (`GameplayStatics.PlaySound2D` "/Game/son/Fire01.Fire01" 0.2)
  (`self.Hit`))

(event `self.Box.OnComponentBeginOverlap`
  (params (OtherActor :type "Actor Object Reference") (OtherComp :type "PrimitiveComponent Object Reference") (OtherBodyIndex :type Integer) (bFromSweep :type Boolean) (SweepResult :type "HitResult Structure (by ref)"))
  (bind _asthe_player_bp (cast `/Game/Blueprint/ThePlayer_BP` OtherActor)))

(event `Hit`
  (for _array_element (`PrimitiveComponent.GetOverlappingActors` (`self.Box`) "/Game/Blueprint/ThePlayer_BP.ThePlayer_BP_C")
    (bind _asthe_player_bp (cast `/Game/Blueprint/ThePlayer_BP` _array_element))
    (`ThePlayer.PlayerTakeDamage` _asthe_player_bp (`self.damage`)))
  (`KismetSystemLibrary.Delay` 0.1)
  (`self.Hit`))

(fn `UserConstructionScript`)